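; GM_Test is an Island Escape game mode that sets up local multiplayer characters, apparently for testing, since it hardcodes AddPlayer(1).
; BeginPlay spawns and possesses an IE_Character per occupied controller slot, tinting and slightly offsetting each by slot, with movement locked.
; The IE_Camera's GameReady event triggers CPartez, which shows the InGame widget, unlocks movement and restores energy from IE_GameInstance.
; SaveCurrentEnergy writes each character's energy back to that instance.
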(event Custom|CPartez
  ;[1 1 1] Finish setup after cinematic
  (bind _returnvalue (UserInterface|CreateWidget "/Game/IslandEscape/UI/InGame.InGame_C"))
  (UserInterface|Viewport|AddtoViewport _returnvalue 0)
  (for _index (range 0 3)
    (bind _asmy_player_controller (Utilities|Casting|CastToMyPlayerController (Game|GetPlayerController _index)))
    (Variables|/Game/IslandEscape/MyPlayerController.MyPlayerController_C|SetMovementAllowed _asmy_player_controller true)
    (bind _asie_character (Utilities|Casting|CastToIE_Character (Pawn|GetControlledPawn _asmy_player_controller)))
    (bind _asie_game_instance (Utilities|Casting|CastToIE_GameInstance (Game|GetGameInstance)))
    (bind _slot (Default|GetControllerSlot _asie_game_instance _index))
    (Variables|/Game/IslandEscape/Character/IE_Character.IE_Character_C|SetCurrentEnergy _asie_character (Utilities|Array|Get(acopy) (Variables|/Game/IslandEscape/IE_GameInstance.IE_GameInstance_C|GetPlayersEnergies _asie_game_instance) _slot))))

(event EventBeginPlay
  (Utilities|FlowControl|Sequence
    (:then_0
      (bind _asie_game_instance (Utilities|Casting|CastToIE_GameInstance (Game|GetGameInstance)))
      (Default|AddPlayer _asie_game_instance 1))
    (:then_1
      ;[1 1 1] Instantiate pawns
      (bind _asie_game_instance_2 (Utilities|Casting|CastToIE_GameInstance (Game|GetGameInstance)))
      (for _index (range 1 (Variables|/Game/IslandEscape/IE_GameInstance.IE_GameInstance_C|GetMaxPlayers _asie_game_instance_2))
        (bind _slot (Default|GetControllerSlot _asie_game_instance_2 (- _index 1)))
        (if (!= _slot -1)
          (bind _returnvalue (Game|SpawnActorfromClass "/Game/IslandEscape/Character/IE_Character.IE_Character_C" (Transformation|GetActorTransform (Class|GameModeBase|FindPlayerStart)) "Undefined" 0 0))
          (bind _asmy_player_controller (Utilities|Casting|CastToMyPlayerController (Game|GetPlayerController (- _index 1))))
          (Variables|/Game/IslandEscape/MyPlayerController.MyPlayerController_C|SetMovementAllowed _asmy_player_controller false)
          (Pawn|Possess (Game|GetPlayerController (- _index 1)) _returnvalue)
          (switch int _slot
            (:0
              (Sprite|SetSpriteColor (Actor|GetComponentbyClass _returnvalue "/Script/Paper2D.PaperFlipbookComponent") "(R=1.000000,G=0.000000,B=0.000000,A=1.000000)"))
            (:1
              (Sprite|SetSpriteColor (Actor|GetComponentbyClass _returnvalue "/Script/Paper2D.PaperFlipbookComponent") "(R=0.000000,G=0.000000,B=1.000000,A=1.000000)"))
            (:2
              (Sprite|SetSpriteColor (Actor|GetComponentbyClass _returnvalue "/Script/Paper2D.PaperFlipbookComponent") "(R=1.000000,G=1.000000,B=0.000000,A=1.000000)"))
            (:3
              (Sprite|SetSpriteColor (Actor|GetComponentbyClass _returnvalue "/Script/Paper2D.PaperFlipbookComponent") "(R=0.000000,G=1.000000,B=0.000000,A=1.000000)")))
          (Transformation|SetWorldLocation (Variables|/Script/Engine.Actor|GetRootComponent _returnvalue) (+ (Transformation|GetWorldLocation (Variables|/Script/Engine.Actor|GetRootComponent _returnvalue)) (Math|Vector|MakeVector (* _slot 0.2) 0.0 0.0)) false true))))
    (:then_2
      ;[1 1 1] Finish setup after cinematic
      (bind _outactors (Actor|GetAllActorsOfClass "/Game/IslandEscape/Camera/IE_Camera.IE_Camera_C"))
      (if (== (Utilities|Array|Length _outactors) 1)
        (EventDispatchers|BindEventtoGameReady (Utilities|Array|Get(acopy) _outactors) (delegate Custom|CPartez))))))

(fn ConstructionScript)

(fn SaveCurrentEnergy
  (bind _asie_game_instance (Utilities|Casting|CastToIE_GameInstance (Game|GetGameInstance)))
  (for (_array_element _array_index) (Variables|/Game/IslandEscape/IE_GameInstance.IE_GameInstance_C|GetPlayers _asie_game_instance)
    (if (!= _array_element -1)
      (bind _asie_character (Utilities|Casting|CastToIE_Character (Game|Player|GetPlayerPawn _array_element)))
      (Utilities|Array|SetArrayElem (Variables|/Game/IslandEscape/IE_GameInstance.IE_GameInstance_C|GetPlayersEnergies _asie_game_instance) _array_index (Variables|/Game/IslandEscape/Character/IE_Character.IE_Character_C|GetCurrentEnergy _asie_character)))))