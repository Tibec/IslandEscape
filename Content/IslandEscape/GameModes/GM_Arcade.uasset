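; Arcade game mode for Island Escape that runs a local multiplayer last-player-standing match.
; BeginPlay spawns and possesses color-tinted characters at slot-named player starts, then runs a camera intro that player button input can stop via CinematicUI.
; When the camera signals ready, the HUD appears, gameplay unlocks and energies load from the GameInstance, which SaveCurrentEnergy writes.
; A Tick state machine detects the sole survivor, swaps music to a jingle, shows the winner and returns to MainMenu.
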(event Custom|CPartez
  ;[1 1 1] Finish setup after cinematic
  (Widget|RemovefromParent (stale EventBeginPlay _returnvalue_2))
  (bind _returnvalue (UserInterface|CreateWidget "/Game/IslandEscape/UI/InGameArcade.InGameArcade_C"))
  (UserInterface|Viewport|AddtoViewport _returnvalue 0)
  (for _index (range 0 3)
    (bind _asmy_player_controller (Utilities|Casting|CastToMyPlayerController (Game|GetPlayerController _index)))
    (Variables|/Game/IslandEscape/MyPlayerController.MyPlayerController_C|SetGameplayStopped _asmy_player_controller false)
    (bind _asie_character (Utilities|Casting|CastToIE_Character (Pawn|GetControlledPawn _asmy_player_controller)))
    (bind _asie_game_instance (Utilities|Casting|CastToIE_GameInstance (Game|GetGameInstance)))
    (bind _slot (Default|GetControllerSlot _asie_game_instance _index))
    (Variables|/Game/IslandEscape/Character/IE_Character.IE_Character_C|SetCurrentEnergy _asie_character (Utilities|Array|Get(acopy) (Variables|/Game/IslandEscape/IE_GameInstance.IE_GameInstance_C|GetPlayersEnergies _asie_game_instance) _slot))))

(event Custom|CustomEvent_0
  (params (SelfReference :type My%20Player%20Controller%20Object%20Reference) (InputAction :type IE_CharacterInput%20Enum :default "NewEnumerator15"))
  ;[1 1 1] Finish setup after cinematic
  (Default|CallInput (stale EventBeginPlay _returnvalue_2) true))

(event Custom|CustomEvent_1
  (params (SelfReference :type My%20Player%20Controller%20Object%20Reference) (Button :type IE_CharacterInput%20Enum :default "NewEnumerator15"))
  ;[1 1 1] Finish setup after cinematic
  (Default|CallInput (stale EventBeginPlay _returnvalue_2) false))

(event Custom|CustomEvent_2
  ;[1 1 1] Finish setup after cinematic
  (bind _outactors (Actor|GetAllActorsOfClass "/Game/IslandEscape/Camera/IE_Camera.IE_Camera_C"))
  (for _array_element _outactors
    (Default|CallStopCinematic _array_element)
    (EventDispatchers|UnbindEventfromFilled (stale EventBeginPlay _returnvalue_2) (delegate Custom|CustomEvent_2))))

(event EventBeginPlay
  (Utilities|FlowControl|Sequence
    (:then_0
      ;[1 1 1] Instantiate pawns
      (bind _asie_game_instance (Utilities|Casting|CastToIE_GameInstance (Game|GetGameInstance)))
      (for _index (range 1 (Variables|/Game/IslandEscape/IE_GameInstance.IE_GameInstance_C|GetMaxPlayers _asie_game_instance))
        (bind _slot (Default|GetControllerSlot _asie_game_instance (- _index 1)))
        (if (!= _slot -1)
          (bind _returnvalue (Game|SpawnActorfromClass "/Game/IslandEscape/Character/IE_Character.IE_Character_C" (Transformation|GetActorTransform (Class|GameModeBase|FindPlayerStart 0 (Utilities|String|ToString(Integer) _slot))) "Undefined" 0 0))
          (Variables|/Game/IslandEscape/Character/IE_Character.IE_Character_C|SetIsArcadeMode _returnvalue true)
          (bind _asmy_player_controller (Utilities|Casting|CastToMyPlayerController (Game|GetPlayerController (- _index 1))))
          (Variables|/Game/IslandEscape/MyPlayerController.MyPlayerController_C|SetMovementAllowed _asmy_player_controller false)
          (Pawn|Possess (Game|GetPlayerController (- _index 1)) _returnvalue)
          (switch int _slot
            (:0
              (Sprite|SetSpriteColor (Actor|GetComponentbyClass _returnvalue "/Script/Paper2D.PaperFlipbookComponent") "(R=1.000000,G=0.000000,B=0.000000,A=1.000000)"))
            (:1
              (Sprite|SetSpriteColor (Actor|GetComponentbyClass _returnvalue "/Script/Paper2D.PaperFlipbookComponent") "(R=0.000000,G=0.000000,B=1.000000,A=1.000000)"))
            (:2
              (Sprite|SetSpriteColor (Actor|GetComponentbyClass _returnvalue "/Script/Paper2D.PaperFlipbookComponent") "(R=1.000000,G=1.000000,B=0.000000,A=1.000000)"))
            (:3
              (Sprite|SetSpriteColor (Actor|GetComponentbyClass _returnvalue "/Script/Paper2D.PaperFlipbookComponent") "(R=0.000000,G=1.000000,B=0.000000,A=1.000000)")))
          (Transformation|SetWorldLocation (Variables|/Script/Engine.Actor|GetRootComponent _returnvalue) (+ (Transformation|GetWorldLocation (Variables|/Script/Engine.Actor|GetRootComponent _returnvalue)) (Math|Vector|MakeVector (* _slot 0.2) (* _slot -75.0) 0.0)) false true))))
    (:then_1
      ;[1 1 1] Finish setup after cinematic
      (bind _outactors (Actor|GetAllActorsOfClass "/Game/IslandEscape/Camera/IE_Camera.IE_Camera_C"))
      (if (== (Utilities|Array|Length _outactors) 1)
        (EventDispatchers|BindEventtoGameReady (Utilities|Array|Get(acopy) _outactors) (delegate Custom|CPartez))
        (bind _returnvalue_2 (UserInterface|CreateWidget "/Game/IslandEscape/UI/CinematicUI.CinematicUI_C"))
        (UserInterface|Viewport|AddtoViewport _returnvalue_2 0)
        (for _index_2 (range 0 4)
          (bind _asie_game_instance_2 (Utilities|Casting|CastToIE_GameInstance (Game|GetGameInstance)))
          (bind _isactive_ (Default|IsPlayerActive _asie_game_instance_2 _index_2))
          (if _isactive_
            (bind _asmy_player_controller_2 (Utilities|Casting|CastToMyPlayerController (Game|GetPlayerController _index_2)))
            (EventDispatchers|BindEventtoButtonPressed _asmy_player_controller_2 (delegate Custom|CustomEvent_0))
            (EventDispatchers|BindEventtoButtonReleased _asmy_player_controller_2 (delegate Custom|CustomEvent_1))
            (EventDispatchers|BindEventtoFilled _returnvalue_2 (delegate Custom|CustomEvent_2))))))))

(event EventTick
  (params (DeltaSeconds :type Float%20%28single-precision%29))
  (switch int (Variables|Default|GetState)
    (:Default
      ;[1 1 1] Check Game Ended
      (Variables|Default|SetAlivePlayerCount 0 :!label _label)
      (bind _outactors (Actor|GetAllActorsOfClass "/Game/IslandEscape/Character/IE_Character.IE_Character_C"))
      (for (_array_element _array_index) _outactors
        (bind _asmy_player_controller (Utilities|Casting|CastToMyPlayerController (Pawn|GetController _array_element)))
        (if (not (Variables|/Game/IslandEscape/MyPlayerController.MyPlayerController_C|GetIsDead _asmy_player_controller))
          (Math|Integer|IncrementInt (Variables|Default|GetAlivePlayerCount)
            (:%20%20
              (Variables|Default|SetLastPlayerAliveId _array_index)))))
      (if (== (Variables|Default|GetAlivePlayerCount) 1)
        (Variables|Default|SetState 1)))
    (:0
      (goto _label))
    (:1
      (Utilities|FlowControl|DoOnce false
        (:Completed
          (bind _outactors_2 (Actor|GetAllActorsOfClass "/Script/Engine.AmbientSound"))
          (for _array_element_2 _outactors_2
            (Audio|Components|Audio|FadeOut (Variables|/Script/Engine.AmbientSound|GetAudioComponent _array_element_2) 1.0 0.0 :!class /Script/Engine.AudioComponent)
            (Utilities|FlowControl|Delay 1.5)
            (Variables|Default|SetState 2)))))
    (:2
      (Utilities|FlowControl|DoOnce false
        (:Completed
          (bind _outactors_3 (Actor|GetAllActorsOfClass "/Script/Engine.AmbientSound"))
          (for _array_element_3 _outactors_3
            (Audio|Components|Audio|SetSound (Variables|/Script/Engine.AmbientSound|GetAudioComponent _array_element_3) "/Game/IslandEscape/Music/ArcadeJingle.ArcadeJingle")
            (Audio|Components|Audio|FadeIn (Variables|/Script/Engine.AmbientSound|GetAudioComponent _array_element_3) 0.0 1.0 0.0 :!class /Script/Engine.AudioComponent)
            (bind _returnvalue (UserInterface|CreateWidget "/Game/IslandEscape/UI/ArcadeWin.ArcadeWin_C"))
            (Default|SetWinner _returnvalue (Variables|Default|GetLastPlayerAliveId))
            (UserInterface|Viewport|AddtoViewport _returnvalue 5000)
            (Utilities|FlowControl|Delay 1e+01)
            (Variables|Default|SetState 3)
            (Default|FadeOut _returnvalue)))))
    (:3
      (Utilities|FlowControl|DoOnce false
        (:Completed
          (bind _outactors_4 (Actor|GetAllActorsOfClass "/Script/Engine.AmbientSound"))
          (for _array_element_4 _outactors_4
            (Audio|Components|Audio|FadeOut (Variables|/Script/Engine.AmbientSound|GetAudioComponent _array_element_4) 1.0 0.0 :!class /Script/Engine.AudioComponent)
            (Utilities|FlowControl|Delay 1.0)
            (Game|OpenLevel(byName) "MainMenu")))))))

(fn ConstructionScript)

(fn SaveCurrentEnergy
  (bind _asie_game_instance (Utilities|Casting|CastToIE_GameInstance (Game|GetGameInstance)))
  (for (_array_element _array_index) (Variables|/Game/IslandEscape/IE_GameInstance.IE_GameInstance_C|GetPlayers _asie_game_instance)
    (if (!= _array_element -1)
      (bind _asie_character (Utilities|Casting|CastToIE_Character (Game|Player|GetPlayerPawn _array_element)))
      (Utilities|Array|SetArrayElem (Variables|/Game/IslandEscape/IE_GameInstance.IE_GameInstance_C|GetPlayersEnergies _asie_game_instance) _array_index (Variables|/Game/IslandEscape/Character/IE_Character.IE_Character_C|GetCurrentEnergy _asie_character)))))