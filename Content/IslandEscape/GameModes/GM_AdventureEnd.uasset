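; Game mode for the end of an Island Escape adventure, showing player results and then the leaderboard before returning to the main menu.
; ComputeResults builds a time-ordered list from the game instance's player times, flagging new records, to fill the Results widget.
; Controller button events, mapped through DetectInputType, drive that widget per player slot.
; Tick polls for readiness, saves named records, swaps in the highlighted leaderboard and rebinds input to press-to-continue.
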(event Custom|SendInput
  (params (SelfReference :type My%20Player%20Controller%20Object%20Reference) (InputAction :type IE_CharacterInput%20Enum :default "NewEnumerator15"))
  (bind _returnvalue (Class|GameplayStatics|GetPlayerControllerID SelfReference))
  (bind _slot (Default|GetControllerSlot (stale EventBeginPlay _asie_game_instance) _returnvalue))
  (if (!= _slot -1)
    (Utilities|DetectInputType InputAction
      (:Start
        (Default|PressStart (stale EventBeginPlay _returnvalue) _slot))
      (:A
        (Default|PressA (stale EventBeginPlay _returnvalue) _slot))
      (:B
        (Default|PressB (stale EventBeginPlay _returnvalue) _slot))
      (:Stick
        (if (Utilities|Enum|NotEqual(Enum) (Variables|Default|GetLastStickInput) InputAction)
          (Variables|Default|SetLastStickInput InputAction)
          (Default|PressStick (stale EventBeginPlay _returnvalue) _slot InputAction))))))

(event Custom|PressToContinue
  (params (SelfReference :type My%20Player%20Controller%20Object%20Reference) (InputAction :type IE_CharacterInput%20Enum :default "NewEnumerator15"))
  (Utilities|DetectInputType InputAction
    (:Start
      _)
    (:A
      _)
    (:B
      _)
    (:Other
      _))
  (Variables|Default|SetGetBackToMenu true))

(event EventBeginPlay
  (Utilities|FlowControl|Sequence
    (:then_0
      (bind _returnvalue (UserInterface|CreateWidget "/Game/IslandEscape/UI/Results.Results_C"))
      (UserInterface|Viewport|AddtoViewport _returnvalue 0)
      (Variables|Default|SetActiveUI _returnvalue))
    (:then_1
      (bind _results (CallFunction|ComputeResults)))
    (:then_2
      (bind _asie_game_instance (Utilities|Casting|CastToIE_GameInstance (Game|GetGameInstance)))
      (for (_array_element _array_index) (Variables|/Game/IslandEscape/IE_GameInstance.IE_GameInstance_C|GetPlayers _asie_game_instance)
        (Default|DisplayPlayer _returnvalue _array_element (!= _array_element -1))
        (bind _asmy_player_controller (Utilities|Casting|CastToMyPlayerController (Game|GetPlayerController _array_index)))
        (EventDispatchers|BindEventtoButtonPressed _asmy_player_controller (delegate Custom|SendInput))
        (bind _array_element_2 (Utilities|Array|ForEachLoopwithBreak _results :!label _label)
          (:LoopBody
            (if (== (.Slot (Utilities|Struct|BreakPlayerResultInfo _array_element_2)) _array_index)
              (Default|SetPlayerResult _returnvalue (.Slot (Utilities|Struct|BreakPlayerResultInfo _array_element_2)) (.Rank (Utilities|Struct|BreakPlayerResultInfo _array_element_2)) (.Time (Utilities|Struct|BreakPlayerResultInfo _array_element_2)) (.IsNewRecord (Utilities|Struct|BreakPlayerResultInfo _array_element_2)))
              (Variables|/Game/IslandEscape/MyPlayerController.MyPlayerController_C|SetGameplayStopped _asmy_player_controller false)
              (goto _label Break))))))))

(event EventTick
  (params (DeltaSeconds :type Float%20%28single-precision%29))
  (if (== (Utilities|GetClass (Variables|Default|GetActiveUI)) "/Game/IslandEscape/UI/Results.Results_C")
    (bind _asresults (Utilities|Casting|CastToResults (Variables|Default|GetActiveUI)))
    (bind _yes (Default|ReadytoContinue _asresults))
    (if _yes
      (for _array_element (stale EventBeginPlay _results)
        (bind _name (Default|GetName _asresults (.Slot (Utilities|Struct|BreakPlayerResultInfo _array_element))))
        (if (.IsNewRecord (Utilities|Struct|BreakPlayerResultInfo _array_element))
          (bind _slot (Default|AddNewRecord (Variables|/Game/IslandEscape/IE_GameInstance.IE_GameInstance_C|GetLeaderboard (stale EventBeginPlay _asie_game_instance)) _name (.Time (Utilities|Struct|BreakPlayerResultInfo _array_element))))
          (Utilities|Array|Add (Variables|Default|GetscoreToHighlight) _slot)))
      (Widget|RemovefromParent _asresults)
      (bind _returnvalue (UserInterface|CreateWidget "/Game/IslandEscape/UI/LeaderBoard.LeaderBoard_C"))
      (UserInterface|Viewport|AddtoViewport _returnvalue 0)
      (Variables|Default|SetActiveUI _returnvalue)
      (bind _asie_game_instance (Utilities|Casting|CastToIE_GameInstance (Game|GetGameInstance)))
      (for _array_element_2 (Variables|/Game/IslandEscape/IE_GameInstance.IE_GameInstance_C|GetPlayers _asie_game_instance)
        (bind _asmy_player_controller (Utilities|Casting|CastToMyPlayerController (Game|GetPlayerController _array_element_2)))
        (EventDispatchers|UnbindEventfromButtonPressed _asmy_player_controller (delegate Custom|SendInput))
        (EventDispatchers|BindEventtoButtonPressed _asmy_player_controller (delegate Custom|PressToContinue)))
      (for _array_element_3 (Variables|Default|GetscoreToHighlight)
        (Default|Highlight _returnvalue _array_element_3)))
    (elif (== (Utilities|GetClass (Variables|Default|GetActiveUI)) "/Game/IslandEscape/UI/LeaderBoard.LeaderBoard_C")
      (if (Variables|Default|GetGetBackToMenu)
        (Game|OpenLevel(byName) "MainMenu")))))

(fn ConstructionScript)

(fn ComputeResults
  (bind _res (LocalVariables|Getres))
  (bind _asie_game_instance (Utilities|Casting|CastToIE_GameInstance (Game|GetGameInstance)))
  (for (_array_element _array_index) (Variables|/Game/IslandEscape/IE_GameInstance.IE_GameInstance_C|GetPlayers _asie_game_instance)
    (if (!= _array_element -1)
      (if (!= (Utilities|Array|Length (LocalVariables|Getres)) 0)
        (for (_array_element_2 _array_index_2) (LocalVariables|Getres)
          (if (> (.Time (Utilities|Struct|BreakPlayerResultInfo _array_element_2)) (Utilities|Array|Get(acopy) (Variables|/Game/IslandEscape/IE_GameInstance.IE_GameInstance_C|GetPlayersTime _asie_game_instance) _array_index))
            (bind _yes (Default|IsNewRecord (Variables|/Game/IslandEscape/IE_GameInstance.IE_GameInstance_C|GetLeaderboard _asie_game_instance) (Utilities|Array|Get(acopy) (Variables|/Game/IslandEscape/IE_GameInstance.IE_GameInstance_C|GetPlayersTime _asie_game_instance) _array_index)))
            (Utilities|Array|SetArrayElem (LocalVariables|Getres) _array_index_2 (Utilities|Struct|MakePlayerResultInfo (.Slot (Utilities|Struct|BreakPlayerResultInfo _array_element_2)) (.Rank (Utilities|Struct|BreakPlayerResultInfo _array_element_2)) (.Time (Utilities|Struct|BreakPlayerResultInfo _array_element_2)) (.IsNewRecord (Utilities|Struct|BreakPlayerResultInfo _array_element_2))))
            (Utilities|Array|Insert (LocalVariables|Getres) (Utilities|Struct|MakePlayerResultInfo _array_index (.Rank (Utilities|Struct|BreakPlayerResultInfo _array_element_2)) (Utilities|Array|Get(acopy) (Variables|/Game/IslandEscape/IE_GameInstance.IE_GameInstance_C|GetPlayersTime _asie_game_instance) _array_index) _yes) _array_index_2)))
        (else
          (bind _yes_2 (Default|IsNewRecord (Variables|/Game/IslandEscape/IE_GameInstance.IE_GameInstance_C|GetLeaderboard _asie_game_instance) (Utilities|Array|Get(acopy) (Variables|/Game/IslandEscape/IE_GameInstance.IE_GameInstance_C|GetPlayersTime _asie_game_instance) _array_index)))
          (Utilities|Array|Insert (LocalVariables|Getres) (Utilities|Struct|MakePlayerResultInfo 0 1 (Utilities|Array|Get(acopy) (Variables|/Game/IslandEscape/IE_GameInstance.IE_GameInstance_C|GetPlayersTime _asie_game_instance) _array_index) _yes_2))))
      (else
        (Utilities|Array|Insert _res (Utilities|Struct|MakePlayerResultInfo _array_index 0 999999.0 false) (- (Utilities|Array|Length _res) 1)))))
  (return (LocalVariables|Getres)))