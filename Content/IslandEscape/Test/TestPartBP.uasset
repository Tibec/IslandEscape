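; TestPartBP is a test actor that moves a particle effect along a spline over a set duration, then fades it out and destroys itself.
; On BeginPlay it gives ParticleSystem1 a dynamic material instance.
; Tick positions the effect by elapsed-time fraction of the spline length, then nearly freezes it via custom time dilation.
; The fade lowers the Opacity parameter by a fixed per-frame step until it drops below zero.
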(event EventBeginPlay
  (bind _particlesystem1 (Variables|Default|GetParticleSystem1))
  (Variables|Default|SetinternalDuration 0.0)
  (bind _returnvalue (Rendering|Material|CreateDynamicMaterialInstance _particlesystem1 0 (Rendering|Material|GetMaterial (Variables|Default|GetParticleSystem1) 0) :!class /Script/Engine.PrimitiveComponent))
  (Rendering|Material|SetMaterial _particlesystem1 0 _returnvalue))

(event EventTick
  (params (DeltaSeconds :type Float%20%28single-precision%29))
  (bind _particlepath (Variables|Default|GetParticlePath))
  (bind _duration (Variables|Default|GetDuration))
  (if (Variables|Default|Getwerefading)
    (bind _returnvalue (Rendering|Material|GetScalarParameterValue (stale EventBeginPlay _returnvalue) "Opacity" :!class /Script/Engine.MaterialInstanceDynamic))
    (Rendering|Material|SetScalarParameterValue (stale EventBeginPlay _returnvalue) "Opacity" (- _returnvalue 0.15) :!class /Script/Engine.MaterialInstanceDynamic)
    (if (not (>= (- _returnvalue 0.15) 0.0))
      (Actor|DestroyActor))
    (else
      (Variables|Default|SetinternalDuration (+ (Variables|Default|GetinternalDuration) DeltaSeconds))
      (if (< (Variables|Default|GetinternalDuration) _duration)
        (Transformation|SetWorldLocation (Variables|Default|GetParticleSystem1) (Spline|GetLocationatDistanceAlongSpline _particlepath (* (/ (Variables|Default|GetinternalDuration) _duration) (Spline|GetSplineLength _particlepath)) "World") false false) ; Move the particle effect along the spline
        (else
          (Variables|/Script/Engine.ParticleSystemComponent|SetCustomTimeDilation (Variables|Default|GetParticleSystem1) 0.001)
          (Variables|Default|Setwerefading true))))))

(fn ConstructionScript)